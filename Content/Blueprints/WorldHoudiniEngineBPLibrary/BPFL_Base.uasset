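; Blueprint function library of helpers for exchanging mesh geometry and attribute data with a Houdini Engine session.
; Setup functions set part info and upload positions, normals, UVs, tangents, per-primitive section indices and the vertex list to a node.
; Vectors are flattened to float lists with Y/Z swapped, positions scaled from centimeters to meters and UV Y flipped.
; Getters read float, int or string attributes by fetching attribute info then data, returning combined success.
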(fn HoudiniCreateandSetPartInfo
  (params (HoudiniSession :type Houdini%20Session%20Structure) (NodeId :type Integer) (FaceCount :type Integer) (VertexCount :type Integer) (PointCount :type Integer) (HoudiniPartType :type EHoudiniPartType%20Enum :default "HOUDINI_PARTTYPE_MESH"))
  (Class|WorldHoudiniEngineBPLibrary|HoudiniSetPartInfo HoudiniSession NodeId (Class|WorldHoudiniEngineBPLibrary|HoudiniCreatePartInfo FaceCount VertexCount PointCount HoudiniPartType)))

(fn HoudiniSetupBaseAttributes
  (params (HoudiniSession :type Houdini%20Session%20Structure) (NodeId :type Integer) (PositionList :type Array%20of%20Vectors) (NormalList :type Array%20of%20Vectors) (UVList :type Array%20of%20Vector%202D%20Structures) (TangentList :type Array%20of%20Vectors) (SectionIndexList :type Array%20of%20Integers) (VertexList :type Array%20of%20Integers))
  (bind _returnvalue (Utilities|Array|Length PositionList))
  (bind _returnvalue_2 (Utilities|Array|Length NormalList))
  (bind _returnvalue_3 (Utilities|Array|Length UVList))
  (bind _returnvalue_4 (Utilities|Array|Length TangentList))
  (bind _returnvalue_5 (Utilities|Array|Length SectionIndexList))
  (Class|WorldHoudiniEngineBPLibrary|HoudiniAddandSetFloatAttribute HoudiniSession NodeId "P" (Class|WorldHoudiniEngineBPLibrary|HoudiniCreateAttributeInfo _returnvalue 3 true "HOUDINI_ATTROWNER_POINT" "HOUDINI_STORAGETYPE_FLOAT") (.FloatList (Class|WorldHoudiniEngineUtilsLibrary|VectorListtoFloatList PositionList true 0.01)) _returnvalue)
  (Class|WorldHoudiniEngineBPLibrary|HoudiniAddandSetFloatAttribute HoudiniSession NodeId "N" (Class|WorldHoudiniEngineBPLibrary|HoudiniCreateAttributeInfo _returnvalue_2 3 true "HOUDINI_ATTROWNER_POINT" "HOUDINI_STORAGETYPE_FLOAT") (.FloatList (Class|WorldHoudiniEngineUtilsLibrary|VectorListtoFloatList NormalList true 1.0)) _returnvalue_2)
  (Class|WorldHoudiniEngineBPLibrary|HoudiniAddandSetFloatAttribute HoudiniSession NodeId "uv" (Class|WorldHoudiniEngineBPLibrary|HoudiniCreateAttributeInfo _returnvalue_3 3 true "HOUDINI_ATTROWNER_POINT" "HOUDINI_STORAGETYPE_FLOAT") (.FloatList (Class|WorldHoudiniEngineUtilsLibrary|Vector2DListtoFloatList UVList true)) _returnvalue_3)
  (Class|WorldHoudiniEngineBPLibrary|HoudiniAddandSetFloatAttribute HoudiniSession NodeId "Tangent" (Class|WorldHoudiniEngineBPLibrary|HoudiniCreateAttributeInfo _returnvalue_4 3 true "HOUDINI_ATTROWNER_POINT" "HOUDINI_STORAGETYPE_FLOAT") (.FloatList (Class|WorldHoudiniEngineUtilsLibrary|VectorListtoFloatList TangentList true 1.0)) _returnvalue_4)
  (Class|WorldHoudiniEngineBPLibrary|HoudiniAddandSetIntAttribute HoudiniSession NodeId "SectionIndex" (Class|WorldHoudiniEngineBPLibrary|HoudiniCreateAttributeInfo _returnvalue_5 1 true "HOUDINI_ATTROWNER_PRIM" "HOUDINI_STORAGETYPE_INT") SectionIndexList _returnvalue_5)
  (Class|WorldHoudiniEngineBPLibrary|HoudiniSetVertexListandFaceCounts HoudiniSession NodeId VertexList))

(fn HoudiniGetFloatAttributeData
  (params (HoudiniSession :type Houdini%20Session%20Structure) (NodeId :type Integer) (PartId :type Integer) (AttributeName :type String) (AttributeOwner :type EHoudiniAttributeOwner%20Enum :default "HOUDINI_ATTROWNER_POINT"))
  (bind (_attribinfo _returnvalue) (Class|WorldHoudiniEngineBPLibrary|HoudiniGetAttributeInfo HoudiniSession NodeId PartId AttributeName AttributeOwner))
  (bind (_dataarray _returnvalue_2) (Class|WorldHoudiniEngineBPLibrary|HoudiniGetAttributeFloatData HoudiniSession NodeId PartId AttributeName _attribinfo))
  (return (and _returnvalue _returnvalue_2) _dataarray))

(fn HoudiniGetIntAttributeData
  (params (HoudiniSession :type Houdini%20Session%20Structure) (NodeId :type Integer) (PartId :type Integer) (AttributeName :type String) (AttributeOwner :type EHoudiniAttributeOwner%20Enum :default "HOUDINI_ATTROWNER_POINT"))
  (bind (_attribinfo _returnvalue) (Class|WorldHoudiniEngineBPLibrary|HoudiniGetAttributeInfo HoudiniSession NodeId PartId AttributeName AttributeOwner))
  (bind (_dataarray _returnvalue_2) (Class|WorldHoudiniEngineBPLibrary|HoudiniGetAttributeIntData HoudiniSession NodeId PartId AttributeName _attribinfo))
  (return (and _returnvalue _returnvalue_2) _dataarray))

(fn HoudiniGetStringAttributeData
  (params (HoudiniSession :type Houdini%20Session%20Structure) (NodeId :type Integer) (PartId :type Integer) (AttributeName :type String) (AttributeOwner :type EHoudiniAttributeOwner%20Enum :default "HOUDINI_ATTROWNER_POINT") (HoudiniSession1 :type Houdini%20Session%20Structure))
  (bind (_attribinfo _returnvalue) (Class|WorldHoudiniEngineBPLibrary|HoudiniGetAttributeInfo HoudiniSession NodeId PartId AttributeName AttributeOwner))
  (bind (_dataarray _returnvalue_2) (Class|WorldHoudiniEngineBPLibrary|HoudiniGetAttributeStringData HoudiniSession1 NodeId PartId AttributeName _attribinfo))
  (return (and _returnvalue_2 _returnvalue) _dataarray))