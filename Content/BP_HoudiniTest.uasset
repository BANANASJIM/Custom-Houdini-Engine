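; Test Blueprint that exercises a Houdini Engine session API through an ActivateSession event; BeginPlay is empty.
; It starts a server session with cook options, loads a digital asset library from a file path and creates its node.
; It then adds a "geo" child node, connects it to the asset's first child and cooks the asset.
; Finally it queries, disconnects and deletes that node, saves a HIP file and cleans up the session.
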(event Custom|Activate%20Session
  (bind _returnvalue (Class|WorldHoudiniEngineBPLibrary|StartSeverandCreateSession (Variables|Default|GetSession)))
  (bind _output_get (Variables|Default|SetSession _returnvalue))
  (bind _returnvalue_2 (Class|WorldHoudiniEngineBPLibrary|CreateHoudiniCookOptions))
  (bind _output_get_2 (Variables|Default|SetHoudiniCookOptions _returnvalue_2))
  (Class|WorldHoudiniEngineBPLibrary|HoudiniInitialize _output_get _output_get_2)
  (if (Class|WorldHoudiniEngineBPLibrary|HoudiniIsInitialize _output_get)
    (bind _assertlibraryid (Class|WorldHoudiniEngineBPLibrary|HoudiniLoadAssertLibraryfromFile _output_get (Variables|Default|GetOtl%20File%20Path) true))
    (bind _output_get_3 (Variables|Default|SetAssert%20Library%20Id _assertlibraryid))
    (bind (_fullopname _label) (Class|WorldHoudiniEngineBPLibrary|HoudiniGetAssertOperatorName _output_get _output_get_3))
    (bind _nodeid (Class|WorldHoudiniEngineBPLibrary|HoudiniCreateNode _output_get _fullopname _label -1 false))
    (bind _childcount (Class|WorldHoudiniEngineBPLibrary|HoudiniComposeChildNodeList _output_get _nodeid "HOUDINI_NODETYPE_ANY" "HOUDINI_NODEFLAGS_ANY" false))
    (bind _childnodeidlist (Class|WorldHoudiniEngineBPLibrary|HoudiniGetComposedChildNodeList _output_get _nodeid _childcount))
    (bind _nodeid_2 (Class|WorldHoudiniEngineBPLibrary|HoudiniCreateNode _output_get "geo" "ProgrammaticBox" _nodeid false))
    (Class|WorldHoudiniEngineBPLibrary|HoudiniConnectNodeInput _output_get _nodeid_2 0 (Utilities|Array|Get(acopy) _childnodeidlist))
    (Class|WorldHoudiniEngineBPLibrary|HoudiniCookNode _output_get _nodeid _output_get_2)
    (Class|WorldHoudiniEngineBPLibrary|HoudiniQueryNodeInput _output_get _nodeid_2)
    (bind _childcount_2 (Class|WorldHoudiniEngineBPLibrary|HoudiniComposeChildNodeList _output_get 0 "HOUDINI_NODETYPE_ANY" "HOUDINI_NODEFLAGS_ANY" false))
    (Class|WorldHoudiniEngineBPLibrary|HoudiniGetComposedChildNodeList _output_get _nodeid _childcount_2)
    (Class|WorldHoudiniEngineBPLibrary|HoudiniDisconnectNodeInput _output_get _nodeid_2)
    (Class|WorldHoudiniEngineBPLibrary|HoudiniDeleteNode _output_get _nodeid_2)
    (Class|WorldHoudiniEngineBPLibrary|HoudiniSaveHIPFile _output_get (Variables|Default|GetHipFilePath) false)
    (Class|WorldHoudiniEngineBPLibrary|HoudiniCleanupSession _output_get)))

(event EventBeginPlay)

(fn ConstructionScript)