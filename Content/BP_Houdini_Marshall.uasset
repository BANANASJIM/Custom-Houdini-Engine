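; Houdini Engine bridge actor that runs a Static Mesh through an HDA from its construction script and displays the result as a procedural mesh.
; It extracts mesh data and materials, marshals them into a Houdini input node, then cooks the connected asset.
; Returned attributes get axis, scale and UV conversion, then triangles split by SectionIndex into material sections.
; The HIP save and session cleanup sit inside the per-section loop.
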(event Custom|Activate
  (bind _proceduralmesh (Variables|Default|GetProceduralMesh))
  (默认|GetMeshData)
  (if (Class|WorldHoudiniEngineBPLibrary|HoudiniIsSessionValid (Variables|Default|GetSession))
    _
    (else
      (bind _returnvalue (Class|WorldHoudiniEngineBPLibrary|StartSeverandCreateSession (Variables|Default|GetSession)))
      (Variables|Default|SetSession _returnvalue)))
  (if (Class|WorldHoudiniEngineBPLibrary|HoudiniIsInitialize (Variables|Default|GetSession))
    _
    (else
      (Class|WorldHoudiniEngineBPLibrary|HoudiniInitialize (Variables|Default|GetSession) (Variables|Default|GetHoudini%20Cook%20Options))))
  (bind _nodeid (Class|WorldHoudiniEngineBPLibrary|HoudiniCreateInputNode (Variables|Default|GetSession) "TestUnrealMesh"))
  (bind _output_get (Variables|Default|SetNode%20Id _nodeid))
  (CallFunction|HoudiniCreateandSetPartInfo (Variables|Default|GetSession) _output_get (Utilities|Array|Length (Variables|Default|GetFace%20List)) (Utilities|Array|Length (Variables|Default|GetVertex%20List)) (Utilities|Array|Length (Variables|Default|GetPosition%20List)) "HOUDINI_PARTTYPE_MESH")
  (CallFunction|HoudiniSetupBaseAttributes (Variables|Default|GetSession) _output_get (Variables|Default|GetPosition%20List) (Variables|Default|GetNormal%20List) (Variables|Default|GetUVList) (Variables|Default|GetTangentList) (Variables|Default|GetSection%20Index%20List) (Variables|Default|GetVertex%20List))
  (Class|WorldHoudiniEngineBPLibrary|HoudiniCommitGeo (Variables|Default|GetSession) _output_get)
  (bind _assertlibraryid (Class|WorldHoudiniEngineBPLibrary|HoudiniLoadAssertLibraryfromFile (Variables|Default|GetSession) (Variables|Default|GetOtl%20File%20Path) false))
  (bind (_fullopname _label) (Class|WorldHoudiniEngineBPLibrary|HoudiniGetAssertOperatorName (Variables|Default|GetSession) _assertlibraryid))
  (bind _nodeid_2 (Class|WorldHoudiniEngineBPLibrary|HoudiniCreateNode :OperatorName _fullopname :Label _label))
  (Class|WorldHoudiniEngineBPLibrary|HoudiniConnectNodeInput (Variables|Default|GetSession) _nodeid_2 0 _output_get)
  (Class|WorldHoudiniEngineBPLibrary|HoudiniCookNode (Variables|Default|GetSession) _nodeid_2 (Variables|Default|GetHoudini%20Cook%20Options))
  (bind _dataarray (CallFunction|HoudiniGetFloatAttributeData (Variables|Default|GetSession) _nodeid_2 0 "P" "HOUDINI_ATTROWNER_POINT"))
  (Variables|Default|SetFinalPosionList (.VectorList (Class|WorldHoudiniEngineUtilsLibrary|FloatListtoVectorList _dataarray true 1e+02)))
  (bind _dataarray_2 (CallFunction|HoudiniGetFloatAttributeData (Variables|Default|GetSession) _nodeid_2 0 "N" "HOUDINI_ATTROWNER_POINT"))
  (Variables|Default|SetFinalNormalList (.VectorList (Class|WorldHoudiniEngineUtilsLibrary|FloatListtoVectorList _dataarray_2 true 1.0)))
  (bind _dataarray_3 (CallFunction|HoudiniGetFloatAttributeData (Variables|Default|GetSession) _nodeid_2 0 "uv" "HOUDINI_ATTROWNER_POINT"))
  (Variables|Default|SetFinalUVList (.Vector2DList (Class|WorldHoudiniEngineUtilsLibrary|FloatListtoVector2DList _dataarray_3 true)))
  (bind _dataarray_4 (CallFunction|HoudiniGetFloatAttributeData (Variables|Default|GetSession) _nodeid_2 0 "Tangent" "HOUDINI_ATTROWNER_POINT"))
  (Variables|Default|SetFianlProcMeshTangentList (.ProcMeshTangentList (Class|WorldHoudiniEngineUtilsLibrary|FloatListtoProcMeshTangentList _dataarray_4 true false)))
  (bind _dataarray_5 (CallFunction|HoudiniGetIntAttributeData (Variables|Default|GetSession) _nodeid_2 0 "SectionIndex" "HOUDINI_ATTROWNER_PRIM"))
  (bind _output_get_2 (Variables|Default|SetSection%20Index%20List _dataarray_5))
  (bind _output_get_3 (Variables|Default|SetFinalVertexList (.VertexList (Class|WorldHoudiniEngineBPLibrary|HoudiniGetVertexList (Variables|Default|GetSession) _nodeid_2 0 (* (.FaceCount (Class|WorldHoudiniEngineBPLibrary|HoudiniGetPartInfoSubData (.PartInfo (Class|WorldHoudiniEngineBPLibrary|HoudiniGetPartInfo (Variables|Default|GetSession) _nodeid_2)))) 3)))))
  (for (_array_element _array_index) (.SplittedVertexLists (Class|WorldHoudiniEngineUtilsLibrary|SplitVertexList _output_get_3 _output_get_2))
    (Class|ProceduralMeshComponent|CreateMeshSectionLinearColor _proceduralmesh _array_index (Variables|Default|GetFinalPosionList) (Utilities|Struct|BreakVertexListStruct _array_element) (Variables|Default|GetFinalNormalList) (Variables|Default|GetFinalUVList) 0 0 0 0 (Variables|Default|GetFianlProcMeshTangentList) false)
    (Rendering|Material|SetMaterial _proceduralmesh _array_index (Utilities|Array|Get(acopy) (Variables|Default|GetMaterial%20List) _array_index))
    (Class|WorldHoudiniEngineBPLibrary|HoudiniSaveHIPFile (Variables|Default|GetSession) (Variables|Default|GetFile%20Path) true)
    (Class|WorldHoudiniEngineBPLibrary|HoudiniCleanupSession (Variables|Default|GetSession))))

(fn ConstructionScript
  (CallFunction|Activate))

(fn GetMeshData
  (bind _staticmesh (Variables|Default|GetStaticMesh))
  (bind (_positionlist _vertexlist _facelist _normallist _tangentlist _uvlist _sectionindexlist _materiallist _returnvalue) (Class|WorldHoudiniEngineUtilsLibrary|GetUnrealMeshData _staticmesh))
  (if _returnvalue
    (Variables|Default|SetPosition%20List _positionlist)
    (Variables|Default|SetVertex%20List _vertexlist)
    (Variables|Default|SetFace%20List _facelist)
    (Variables|Default|SetNormal%20List _normallist)
    (Variables|Default|SetTangentList _tangentlist)
    (Variables|Default|SetUVList _uvlist)
    (Variables|Default|SetSection%20Index%20List _sectionindexlist)
    (Variables|Default|SetMaterial%20List _materiallist)))